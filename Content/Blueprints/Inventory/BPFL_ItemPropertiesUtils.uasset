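; Blueprint function library that generates item property structs from an item quality tier and a skill type.
; Each skill type (missile, beam, area of effect, self) supplies base stats, which a multiplier that doubles with each quality tier then scales.
; Scaling multiplies most stats, caps angle at a full circle, truncates split count and divides interval.
; The scaled struct does not carry over IsChannelled, which the beam base sets.
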(fn GenerateItemProps
  (params (ItemQuality :type E_ItemQuality%20Enum :default "NewEnumerator0") (SkillType :type E_SkillType%20Enum :default "NewEnumerator0"))
  (bind _multiplier (CallFunction|GetMultiplierfromQuality ItemQuality))
  (bind _baseitemprops (CallFunction|GetBaseItemPropsfromSkillType SkillType))
  (bind _multipliedprops (CallFunction|ApplyMultipliertoItemProps _multiplier _baseitemprops))
  (return _multipliedprops))

(fn GetMultiplierfromQuality
  (params (ItemQuality :type E_ItemQuality%20Enum :default "NewEnumerator0"))
  (switch Utilities|FlowControl|Switch|SwitchonE_ItemQuality ItemQuality
    (:NewEnumerator0
      (return 1.0))
    (:NewEnumerator1
      (return 2.0))
    (:NewEnumerator2
      (return 4.0))
    (:NewEnumerator3
      (return 8.0))
    (:NewEnumerator4
      (return 16.0))
    (:NewEnumerator5
      (return 32.0))
    (:NewEnumerator6
      (return 64.0))
    (:NewEnumerator7
      (return 128.0))
    (:NewEnumerator8
      (return 256.0))))

(fn GetBaseItemPropsfromSkillType
  (params (SkillType :type E_SkillType%20Enum :default "NewEnumerator0"))
  (switch Utilities|FlowControl|Switch|SwitchonE_SkillType SkillType
    (:NewEnumerator0
      (return (Utilities|Struct|MakeS_ItemProperties "" "NewEnumerator0" "NewEnumerator0" "NewEnumerator0" 5.0 1e+03 2.5e+02 0.0 0.0 2.0)))
    (:NewEnumerator1
      (return (Utilities|Struct|MakeS_ItemProperties "" "NewEnumerator0" "NewEnumerator0" "NewEnumerator0" 1.0 1e+03 0.0 2.0 0.0 0.5 0.0 0.0 0.0 0 false false true)))
    (:NewEnumerator2
      (return (Utilities|Struct|MakeS_ItemProperties "" "NewEnumerator0" "NewEnumerator0" "NewEnumerator0" 1.0 1e+03 0.0 1e+01 3.6e+02 5.0)))
    (:NewEnumerator3
      (return (Utilities|Struct|MakeS_ItemProperties "" "NewEnumerator0" "NewEnumerator0" "NewEnumerator0" 1.0 0.0 0.0 0.0 0.0 5.0)))))

(fn ApplyMultipliertoItemProps
  (params (Multiplier :type Float%20%28double-precision%29) (ItemProps :type S%20Item%20Properties%20Structure))
  (bind (_name _quality _skilltype _essence _basevalue _range _speed _width _angle _interval _criticalchance _criticalmultiplier _splitchance _splitcount) (Utilities|Struct|BreakS_ItemProperties ItemProps))
  (return (Utilities|Struct|MakeS_ItemProperties "" "NewEnumerator0" "NewEnumerator0" "NewEnumerator0" (* Multiplier _basevalue) (* Multiplier _range) (* Multiplier _speed) (* Multiplier _width) (Math|Float|Clamp(Float) (* Multiplier _angle) 0.0 3.6e+02) (/ _interval Multiplier) (* Multiplier _criticalchance) (* Multiplier _criticalmultiplier) (* Multiplier _splitchance) (Math|Float|Truncate (* _splitcount Multiplier)))))