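; BP_RuneForge is the rune forge Blueprint, which opens its W_RuneForge interface as soon as play begins.
; ShowInterface creates the widget, adds it to the viewport and switches the first player to UI-only input with a visible cursor.
; It then passes its stored essences, maximum essence storage and inventory component to the widget through its register functions.
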(event EventBeginPlay
  (CallFunction|ShowInterface))

(fn ConstructionScript)

(fn ShowInterface
  (bind _returnvalue (Game|GetPlayerController 0))
  (bind _returnvalue_2 (UserInterface|CreateWidget "/Game/UI/W_RuneForge.W_RuneForge_C"))
  (Variables|Default|SetUIWidgetRef _returnvalue_2)
  (UserInterface|Viewport|AddtoViewport _returnvalue_2 0)
  (Input|SetInputModeUIOnly _returnvalue (Variables|Default|GetUIWidgetRef) "DoNotLock" false)
  (Variables|/Script/Engine.PlayerController|SetbShowMouseCursor _returnvalue true)
  (Default|RegisterEssences (Variables|Default|GetUIWidgetRef) (Variables|Default|GetStoredEssence) (Variables|Default|GetMaxEssenceStorage))
  (Default|RegisterInventory (Variables|Default|GetUIWidgetRef) (Variables|Default|GetBP_InventoryComponent)))